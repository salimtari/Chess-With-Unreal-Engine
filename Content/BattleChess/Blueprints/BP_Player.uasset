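; Battle chess player Blueprint that holds the state of both sides, Player and Engine, and controls the board camera.
; Setters rebuild the player structs to update name, color, check and legal-move flags, and move and capture counts.
; SetPlayerCamera eases the camera to the White or Black anchor and resets its azimuth pivot, which RotateCamera yaws.
; CheckCheckmate prints debug text and effectively returns only the check flag, ignoring legal moves.
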(event Custom|SetPlayerCamera
  (params (PlayerColor :type EN_PlayerColor%20Enum :default "NewEnumerator0"))
  (bind _white (Variables|Default|GetWhite))
  (bind _black (Variables|Default|GetBlack))
  (bind _returnvalue (Transformation|GetRelativeTransform _black))
  (bind _returnvalue_2 (Transformation|GetRelativeTransform _white))
  (Components|MoveComponentTo (Variables|Default|GetCameraAzimuth) "0, 0, 0" "0, 0, 0" true true 1.0 true)
  (switch Utilities|FlowControl|Switch|SwitchonEN_PlayerColor PlayerColor
    (:NewEnumerator0
      (Components|MoveComponentTo (Variables|Default|GetCamera) (.location _returnvalue_2) (.rotation _returnvalue_2) true true 3.0 false))
    (:NewEnumerator1
      (Components|MoveComponentTo (Variables|Default|GetCamera) (.location _returnvalue) (.rotation _returnvalue) true true 3.0 false))))

(fn ConstructionScript)

(fn GetPlayerbyIndex
  (params (PlayerIndex :type Integer))
  (if (== PlayerIndex (.index (Variables|Default|GetPlayer)))
    (return (Variables|Default|GetPlayer))
    (else
      (return (Variables|Default|GetEngine)))))

(fn GetPlayerbyColor
  (params (PlayerColor :type EN_PlayerColor%20Enum :default "NewEnumerator0"))
  (if (Utilities|Enum|Equal(Enum) PlayerColor (.color (Variables|Default|GetPlayer)))
    (return (Variables|Default|GetPlayer))
    (else
      (return (Variables|Default|GetEngine)))))

(fn SetPlayerColor
  (params (PlayerIndex :type Integer) (PlayerColor :type EN_PlayerColor%20Enum :default "NewEnumerator0"))
  (switch int PlayerIndex
    (:0
      (Variables|Default|SetPlayer (Utilities|Struct|MakeST_Player (.Name (Utilities|Struct|BreakST_Player (Variables|Default|GetPlayer))) PlayerColor (.Index (Utilities|Struct|BreakST_Player (Variables|Default|GetPlayer))) (.isInCheckFlag (Utilities|Struct|BreakST_Player (Variables|Default|GetPlayer))) (.HasLegalMoves (Utilities|Struct|BreakST_Player (Variables|Default|GetPlayer))) (.MoveCount (Utilities|Struct|BreakST_Player (Variables|Default|GetPlayer))) (.Captures (Utilities|Struct|BreakST_Player (Variables|Default|GetPlayer))))))
    (:1
      (Variables|Default|SetEngine (Utilities|Struct|MakeST_Player (.Name (Utilities|Struct|BreakST_Player (Variables|Default|GetEngine))) PlayerColor (.Index (Utilities|Struct|BreakST_Player (Variables|Default|GetEngine))) (.isInCheckFlag (Utilities|Struct|BreakST_Player (Variables|Default|GetEngine))) (.HasLegalMoves (Utilities|Struct|BreakST_Player (Variables|Default|GetEngine))) (.MoveCount (Utilities|Struct|BreakST_Player (Variables|Default|GetEngine))) (.Captures (Utilities|Struct|BreakST_Player (Variables|Default|GetEngine))))))))

(fn SetPlayerName
  (params (PlayerIndex :type Integer) (PlayerName :type String))
  (switch int PlayerIndex
    (:0
      (Variables|Default|SetPlayer (Utilities|Struct|MakeST_Player PlayerName (.Color (Utilities|Struct|BreakST_Player (Variables|Default|GetPlayer))) (.Index (Utilities|Struct|BreakST_Player (Variables|Default|GetPlayer))) (.isInCheckFlag (Utilities|Struct|BreakST_Player (Variables|Default|GetPlayer))) (.HasLegalMoves (Utilities|Struct|BreakST_Player (Variables|Default|GetPlayer))) (.MoveCount (Utilities|Struct|BreakST_Player (Variables|Default|GetPlayer))) (.Captures (Utilities|Struct|BreakST_Player (Variables|Default|GetPlayer))))))
    (:1
      (Variables|Default|SetEngine (Utilities|Struct|MakeST_Player PlayerName (.Color (Utilities|Struct|BreakST_Player (Variables|Default|GetEngine))) (.Index (Utilities|Struct|BreakST_Player (Variables|Default|GetEngine))) (.isInCheckFlag (Utilities|Struct|BreakST_Player (Variables|Default|GetEngine))) (.HasLegalMoves (Utilities|Struct|BreakST_Player (Variables|Default|GetEngine))) (.MoveCount (Utilities|Struct|BreakST_Player (Variables|Default|GetEngine))) (.Captures (Utilities|Struct|BreakST_Player (Variables|Default|GetEngine))))))))

(fn IncrementPlayerMoveCount
  (params (PlayerIndex :type Integer))
  (switch int PlayerIndex
    (:0
      (Variables|Default|SetPlayer (Utilities|Struct|MakeST_Player (.Name (Utilities|Struct|BreakST_Player (Variables|Default|GetPlayer))) (.Color (Utilities|Struct|BreakST_Player (Variables|Default|GetPlayer))) (.Index (Utilities|Struct|BreakST_Player (Variables|Default|GetPlayer))) (.isInCheckFlag (Utilities|Struct|BreakST_Player (Variables|Default|GetPlayer))) (.HasLegalMoves (Utilities|Struct|BreakST_Player (Variables|Default|GetPlayer))) (+ (.MoveCount (Utilities|Struct|BreakST_Player (Variables|Default|GetPlayer))) 1) (.Captures (Utilities|Struct|BreakST_Player (Variables|Default|GetPlayer))))))
    (:1
      (Variables|Default|SetEngine (Utilities|Struct|MakeST_Player (.Name (Utilities|Struct|BreakST_Player (Variables|Default|GetEngine))) (.Color (Utilities|Struct|BreakST_Player (Variables|Default|GetEngine))) (.Index (Utilities|Struct|BreakST_Player (Variables|Default|GetEngine))) (.isInCheckFlag (Utilities|Struct|BreakST_Player (Variables|Default|GetEngine))) (.HasLegalMoves (Utilities|Struct|BreakST_Player (Variables|Default|GetEngine))) (+ (.MoveCount (Utilities|Struct|BreakST_Player (Variables|Default|GetEngine))) 1) (.Captures (Utilities|Struct|BreakST_Player (Variables|Default|GetEngine))))))))

(fn IncrementPlayerCaptureCount
  (params (PlayerIndex :type Integer))
  (switch int PlayerIndex
    (:0
      (Variables|Default|SetPlayer (Utilities|Struct|MakeST_Player (.Name (Utilities|Struct|BreakST_Player (Variables|Default|GetPlayer))) (.Color (Utilities|Struct|BreakST_Player (Variables|Default|GetPlayer))) (.Index (Utilities|Struct|BreakST_Player (Variables|Default|GetPlayer))) (.isInCheckFlag (Utilities|Struct|BreakST_Player (Variables|Default|GetPlayer))) (.HasLegalMoves (Utilities|Struct|BreakST_Player (Variables|Default|GetPlayer))) (.MoveCount (Utilities|Struct|BreakST_Player (Variables|Default|GetPlayer))) (+ (.Captures (Utilities|Struct|BreakST_Player (Variables|Default|GetPlayer))) 1))))
    (:1
      (Variables|Default|SetEngine (Utilities|Struct|MakeST_Player (.Name (Utilities|Struct|BreakST_Player (Variables|Default|GetEngine))) (.Color (Utilities|Struct|BreakST_Player (Variables|Default|GetEngine))) (.Index (Utilities|Struct|BreakST_Player (Variables|Default|GetEngine))) (.isInCheckFlag (Utilities|Struct|BreakST_Player (Variables|Default|GetEngine))) (.HasLegalMoves (Utilities|Struct|BreakST_Player (Variables|Default|GetEngine))) (.MoveCount (Utilities|Struct|BreakST_Player (Variables|Default|GetEngine))) (+ (.Captures (Utilities|Struct|BreakST_Player (Variables|Default|GetEngine))) 1))))))

(fn SetKinginCheckFlag
  (params (PlayerIndex :type Integer) (IsInCheck :type Boolean))
  (switch int PlayerIndex
    (:0
      (Variables|Default|SetPlayer (Utilities|Struct|MakeST_Player (.Name (Utilities|Struct|BreakST_Player (Variables|Default|GetPlayer))) (.Color (Utilities|Struct|BreakST_Player (Variables|Default|GetPlayer))) (.Index (Utilities|Struct|BreakST_Player (Variables|Default|GetPlayer))) IsInCheck (.HasLegalMoves (Utilities|Struct|BreakST_Player (Variables|Default|GetPlayer))) (.MoveCount (Utilities|Struct|BreakST_Player (Variables|Default|GetPlayer))) (.Captures (Utilities|Struct|BreakST_Player (Variables|Default|GetPlayer))))))
    (:1
      (Variables|Default|SetEngine (Utilities|Struct|MakeST_Player (.Name (Utilities|Struct|BreakST_Player (Variables|Default|GetEngine))) (.Color (Utilities|Struct|BreakST_Player (Variables|Default|GetEngine))) (.Index (Utilities|Struct|BreakST_Player (Variables|Default|GetEngine))) IsInCheck (.HasLegalMoves (Utilities|Struct|BreakST_Player (Variables|Default|GetEngine))) (.MoveCount (Utilities|Struct|BreakST_Player (Variables|Default|GetEngine))) (.Captures (Utilities|Struct|BreakST_Player (Variables|Default|GetEngine))))))))

(fn SetHasLegalMovesFlag
  (params (PlayerIndex :type Integer) (HasLegalMoves :type Boolean))
  (switch int PlayerIndex
    (:0
      (Variables|Default|SetPlayer (Utilities|Struct|MakeST_Player (.Name (Utilities|Struct|BreakST_Player (Variables|Default|GetPlayer))) (.Color (Utilities|Struct|BreakST_Player (Variables|Default|GetPlayer))) (.Index (Utilities|Struct|BreakST_Player (Variables|Default|GetPlayer))) (.isInCheckFlag (Utilities|Struct|BreakST_Player (Variables|Default|GetPlayer))) HasLegalMoves (.MoveCount (Utilities|Struct|BreakST_Player (Variables|Default|GetPlayer))) (.Captures (Utilities|Struct|BreakST_Player (Variables|Default|GetPlayer))))))
    (:1
      (Variables|Default|SetEngine (Utilities|Struct|MakeST_Player (.Name (Utilities|Struct|BreakST_Player (Variables|Default|GetEngine))) (.Color (Utilities|Struct|BreakST_Player (Variables|Default|GetEngine))) (.Index (Utilities|Struct|BreakST_Player (Variables|Default|GetEngine))) (.isInCheckFlag (Utilities|Struct|BreakST_Player (Variables|Default|GetEngine))) HasLegalMoves (.MoveCount (Utilities|Struct|BreakST_Player (Variables|Default|GetEngine))) (.Captures (Utilities|Struct|BreakST_Player (Variables|Default|GetEngine))))))))

(fn RotateCamera
  (params (Axis :type Float%20%28double-precision%29))
  (if (!= Axis 0.0)
    (Transformation|SetRelativeRotation (Variables|Default|GetCameraAzimuth) (Math|Rotator|MakeRotator 0.0 0.0 (+ Axis (.yaw (Variables|/Script/Engine.SceneComponent|GetRelativeRotation (Variables|Default|GetCameraAzimuth))))) false false)))

(fn CheckCheckmate
  (params (Color :type EN_PlayerColor%20Enum :default "NewEnumerator0"))
  (bind _player (GamePlay|GetPlayerbyColor Color))
  (bind (_name _color _index _isincheckflag) (Utilities|Struct|BreakST_Player _player))
  (Development|PrintText (Utilities|Text|FormatText "checkflag: {is in checkflag}" _isincheckflag) true true "(R=0.000000,G=0.660000,B=1.000000,A=1.000000)" 2e+01)
  (Development|PrintText (Utilities|Text|FormatText "legal moves: {is in checkflag}" 0) true true "(R=0.000000,G=0.660000,B=1.000000,A=1.000000)" 2e+01)
  (Development|PrintText (Utilities|Text|FormatText "Color: {is in checkflag}" (Utilities|String|EnumtoString _color)) true true "(R=0.000000,G=0.660000,B=1.000000,A=1.000000)" 2e+01)
  (return (and _isincheckflag (not false))))